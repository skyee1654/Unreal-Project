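; Side-scroller platform that fades away while the character is in its trigger box, then reappears after a recovery delay.
; A timeline, rate-scaled by FadeAwayTime, drives Opacity on a dynamic material instance.
; Leaving before the fade completes reverses it from its current point.
; A completed fade disables mesh collision until RecoveryTime passes, then restores it and reverses the timeline, with flags separating the two directions.
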(event `self.ReceiveBeginPlay`
  (`parent.ReceiveBeginPlay`)
  (bind _returnvalue (`PrimitiveComponent.CreateDynamicMaterialInstance` (`self.PlatformMesh`) 0 "/Game/Materials/M_FadingPlatform.M_FadingPlatform" "None"))
  (set `self.PlatformMaterial` _returnvalue))

(event `self.Box.OnComponentBeginOverlap`
  (params (OverlappedComponent :type "PrimitiveComponent Object Reference") (OtherActor :type "Actor Object Reference") (OtherComp :type "PrimitiveComponent Object Reference") (OtherBodyIndex :type Integer) (bFromSweep :type Boolean) (SweepResult :type "HitResult Structure (by ref)"))
  (cast `/Game/SideScrollerBP/Blueprints/SideScrollerCharacter` OtherActor)
  (`self.BeginFadeAway`))

(event `self.Box.OnComponentEndOverlap`
  (params (OverlappedComponent :type "PrimitiveComponent Object Reference") (OtherActor :type "Actor Object Reference") (OtherComp :type "PrimitiveComponent Object Reference") (OtherBodyIndex :type Integer))
  (cast `/Game/SideScrollerBP/Blueprints/SideScrollerCharacter` OtherActor)
  (`self.EndFadeAway`))

(event `BeginFadeAway`
  (if (not (`self.HasFadedAway?`))
    (set `self.IsFadingAway?` true)
    (`TimelineComponent.SetPlayRate` (`self.FadeAwayAnimation`) (/ 1.0 (`self.Fade Away Time`)))
    (bind (_direction _alpha) (`Timeline|FadeAwayAnimation` :!label _label)
      (:`Update`
        (`MaterialInstanceDynamic.SetScalarParameterValue` (`self.PlatformMaterial`) "Opacity" _alpha))
      (:`Finished`
        (if (`self.IsFadingAway?`)
          (set `self.HasFadedAway?` true)
          (`PrimitiveComponent.SetCollisionEnabled` (`self.PlatformMesh`) "NoCollision")
          (`KismetSystemLibrary.Delay` (`self.RecoveryTime`))
          (`PrimitiveComponent.SetCollisionEnabled` (`self.PlatformMesh`) "QueryAndPhysics")
          (set `self.HasFadedAway?` false)
          (set `self.IsFadingAway?` false :!label _label_2)
          (goto _label :!via `Reverse`))))))

(event `EndFadeAway`
  (if (not (`self.HasFadedAway?`))
    (goto _label_2)))

(fn `UserConstructionScript`
  (`parent.UserConstructionScript`))