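; Moving platform Blueprint that carries its mesh along a spline path in a configurable direction.
; The construction script sets the path's length through its second spline point and rotates it to match the Direction setting.
; On BeginPlay, a timeline played at the inverse of PlatformSpeed lerps distance along the spline, so larger values mean slower travel.
; Each update teleports the mesh to that point without sweeping.
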(event `self.ReceiveBeginPlay`
  (bind _path (`self.Path`))
  (`parent.ReceiveBeginPlay`)
  (`TimelineComponent.SetPlayRate` (`self.BackandForthAnimation`) (/ 1.0 (`self.PlatformSpeed`)))
  (bind (_direction _alpha) (`Timeline|BackandForthAnimation` :!via `PlayFromStart`)
    (:`Update`
      (`SceneComponent.K2_SetWorldLocation` (`self.PlatformMesh`) (`SplineComponent.GetLocationAtDistanceAlongSpline` _path (`KismetMathLibrary.Lerp` 0.0 (`SplineComponent.GetSplineLength` _path) _alpha) "World") false true))))

(fn `UserConstructionScript`
  (bind _path (`self.Path`))
  (`parent.UserConstructionScript`)
  (`SplineComponent.SetLocationAtSplinePoint` (`self.Path`) 1 (`KismetMathLibrary.MakeVector` (`self.SplineLength`)) "Local" true)
  (switch `/Game/Data/Enum_Directions` (`self.Direction`)
    (:`NewEnumerator0`
      (`SceneComponent.K2_SetRelativeRotation` _path (struct :`Pitch` 90.0) false false))
    (:`NewEnumerator1`
      (`SceneComponent.K2_SetRelativeRotation` _path (struct :`Pitch` -90.0) false false))
    (:`NewEnumerator2`
      (`SceneComponent.K2_SetRelativeRotation` _path (struct :`Yaw` 90.0) false false))
    (:`NewEnumerator3`
      (`SceneComponent.K2_SetRelativeRotation` _path (struct :`Yaw` -90.0) false false))))